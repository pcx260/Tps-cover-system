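; Third-person shooter character prototype with wall cover: P runs a cover check and J plays the Reload montage.
; Covertrace casts two side-offset debug line traces along the inverted plane constraint normal to set whether cover continues right or left.
; It then capsule-traces behind the character, snapping it to any hit and storing the surface normal as the movement plane constraint.
; Overlap, Tick and movement input events are empty, with older cover logic left disconnected.
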(event `self. rightcapsule.OnComponentBeginOverlap`
  (params (OverlappedComponent :type "PrimitiveComponent Object Reference") (OtherActor :type "Actor Object Reference") (OtherComp :type "PrimitiveComponent Object Reference") (OtherBodyIndex :type Integer) (bFromSweep :type Boolean) (SweepResult :type "HitResult Structure (by ref)")))

(event `self. rightcapsule.OnComponentEndOverlap`
  (params (OverlappedComponent :type "PrimitiveComponent Object Reference") (OtherActor :type "Actor Object Reference") (OtherComp :type "PrimitiveComponent Object Reference") (OtherBodyIndex :type Integer)))

(event `EnhancedInput|/Game/tps/input/movement`
  (params (ActionValue :type "Vector2D Structure") (ElapsedSeconds :type "Float (double-precision)") (TriggeredSeconds :type "Float (double-precision)") (InputAction :type "InputAction Object Reference" :default "/Game/tps/input/movement.movement")))

(event `Key|J`
  (params (Key :type "Key Structure"))
  (:`Pressed`
    (`self.PlayAnimMontage` "/Game/tps/animation/animations/reload.reload")))

(event `Key|P`
  (params (Key :type "Key Structure")))

(event `self.ReceiveTick`
  (params (DeltaSeconds :type "Float (single-precision)")))

(event `Key|P`
  (params (Key :type "Key Structure"))
  (:`Pressed`
    (`self.covertrace`)))

(fn `covertrace`
  (locals (righthit :type Boolean :default false) (lefthit :type Boolean :default false))
  (bind _returnvalue (`self.K2_GetActorLocation`))
  (bind _planeconstraintnormal (`MovementComponent.PlaneConstraintNormal` (`self.CharacterMovement`)))
  (bind _returnvalue_2 (* (`MovementComponent.PlaneConstraintNormal` (`self.CharacterMovement`)) -1.0))
  (bind _returnvalue_3 (+ (`self.K2_GetActorLocation`) (* (`KismetMathLibrary.GetRightVector` (`KismetMathLibrary.MakeRotFromX` _planeconstraintnormal)) 45.0)))
  (bind _returnvalue_4 (+ (`self.K2_GetActorLocation`) (* (`KismetMathLibrary.GetRightVector` (`KismetMathLibrary.MakeRotFromX` _returnvalue_2)) 45.0)))
  (`|ExecutionSequence`
    (:`then_0`
      (bind (_outhit _returnvalue_5) (`KismetSystemLibrary.LineTraceSingle` :`Start` _returnvalue_4 :`End` (+ _returnvalue_4 (* _returnvalue_2 200.0)) :`TraceChannel` "TraceTypeQuery3" :`DrawDebugType` "ForOneFrame" :`TraceColor` (struct :`G` 0.517368 :`B` 1.0 :`A` 1.0)))
      (bind _output_get (set `local.righthit` _returnvalue_5))
      (if _output_get
        (set `self.bcanright` true)
        (else
          (set `self.bcanright` false))))
    (:`then_1`
      (bind (_outhit_2 _returnvalue_6) (`KismetSystemLibrary.LineTraceSingle` :`Start` _returnvalue_3 :`End` (+ _returnvalue_3 (* (* _planeconstraintnormal -1.0) 200.0)) :`TraceChannel` "TraceTypeQuery3" :`DrawDebugType` "ForOneFrame"))
      (bind _output_get_2 (set `local.lefthit` _returnvalue_6))
      (if _output_get_2
        (set `self.bcanleft` true)
        (else
          (set `self.bcanleft` false))))
    (:`then_2`
      (bind (_outhit_3 _returnvalue_7) (`KismetSystemLibrary.CapsuleTraceSingle` :`Start` _returnvalue :`End` (+ (* (`self.GetActorForwardVector`) -15.0) _returnvalue) :`Radius` 50.0 :`HalfHeight` 30.0 :`TraceChannel` "TraceTypeQuery3" :`DrawDebugType` "ForOneFrame"))
      (if _returnvalue_7
        (bind (_bblockinghit _binitialoverlap _time _distance _location _impactpoint _normal) (`GameplayStatics.BreakHitResult` _outhit_3))
        (`MovementComponent.SetPlaneConstraintNormal` (`self.CharacterMovement`) _normal)
        (`self.K2_SetActorLocation` _location)))))

(fn `UserConstructionScript`)